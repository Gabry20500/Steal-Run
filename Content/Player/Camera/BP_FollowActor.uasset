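; BP_FollowActor is a camera-follow actor for the player, but its runtime follow and view-target logic is unwired and Tick is empty.
; BeginPlay caches the BP_PlayerCharacter, while the construction script positions the actor from PlayerReference and yaws it toward the player.
; The unused update takes X and Z from helper functions, where dead zones act as plain offsets and a nonzero FixedZValue locks height.
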(event `self.ReceiveBeginPlay`
  (bind _returnvalue (`GameplayStatics.GetActorOfClass` (`GameModeBase.DefaultPawnClass` (`GameplayStatics.GetGameMode`))))
  (bind _asbp_player_character (cast `/Game/Player/BP_PlayerCharacter` _returnvalue))
  (set `self.PlayerReference` _asbp_player_character))

(event `self.ReceiveTick`
  (params (DeltaSeconds :type "Float (single-precision)")))

(fn `GetNewXValue`
  (returns (NewX :type "Float (double-precision)"))
  (bind _returnvalue_x (`KismetMathLibrary.BreakVector` (`self.K2_GetActorLocation`)))
  (bind _returnvalue_x_2 (`KismetMathLibrary.BreakVector` (`self.K2_GetActorLocation`)))
  (bind _returnvalue_x_3 (`KismetMathLibrary.BreakVector` (`self.K2_GetActorLocation` (`self.PlayerReference`))))
  (bind _returnvalue_x_4 (`KismetMathLibrary.BreakVector` (`self.K2_GetActorLocation` (`self.PlayerReference`))))
  (bind _returnvalue (- _returnvalue_x_3 (`self.YDeadZone`)))
  (bind _returnvalue_2 (- _returnvalue_x_4 (`self.YDeadZone`)))
  (if (> _returnvalue_2 _returnvalue_x_2)
    (return _returnvalue_2)
    (elif (< _returnvalue _returnvalue_x)
      (return _returnvalue)
      (else
        (return (`self.Camera Y`))))))

(fn `GetNewZValue`
  (returns (`New Z` :type "Float (double-precision)"))
  (bind (_returnvalue_x _returnvalue_y _returnvalue_z) (`KismetMathLibrary.BreakVector` (`self.K2_GetActorLocation`)))
  (bind (_returnvalue_x_2 _returnvalue_y_2 _returnvalue_z_2) (`KismetMathLibrary.BreakVector` (`self.K2_GetActorLocation`)))
  (bind (_returnvalue_x_3 _returnvalue_y_3 _returnvalue_z_3) (`KismetMathLibrary.BreakVector` (`self.K2_GetActorLocation` (`self.PlayerReference`))))
  (bind (_returnvalue_x_4 _returnvalue_y_4 _returnvalue_z_4) (`KismetMathLibrary.BreakVector` (`self.K2_GetActorLocation` (`self.PlayerReference`))))
  (bind _returnvalue (- _returnvalue_z_3 (`self.ZDeadZone`)))
  (bind _returnvalue_2 (- _returnvalue_z_4 (`self.ZDeadZone`)))
  (if (!= (`self.FixedZValue`) 0.0)
    (return (`self.FixedZValue`))
    (elif (> _returnvalue _returnvalue_z)
      (return _returnvalue)
      (elif (< _returnvalue_2 _returnvalue_z_2)
        (return _returnvalue_2)
        (else
          (return (`self.Camera Z`)))))))

(fn `UserConstructionScript`
  (bind (_returnvalue_x _returnvalue_y _returnvalue_z) (`KismetMathLibrary.BreakVector` (`self.K2_GetActorLocation` (`self.PlayerReference`))))
  (bind (_returnvalue_roll _returnvalue_pitch _returnvalue_yaw) (`KismetMathLibrary.BreakRotator` (`KismetMathLibrary.FindLookAtRotation` (`self.K2_GetActorLocation`) (`self.K2_GetActorLocation` (`self.PlayerReference`)))))
  (bind _output_get (set `self.Camera Y` _returnvalue_y))
  (if (!= (`self.FixedZValue`) 0.0)
    (set `self.Camera Z` (`self.FixedZValue`))
    (else
      (bind _output_get_2 (set `self.Camera Z` (+ _returnvalue_z (`self.ZDeadZone`))))))
  (`self.K2_SetActorLocation` (`KismetMathLibrary.MakeVector` (`self.XOffset`) _output_get _output_get_2))
  (`self.K2_SetActorRotation` (`KismetMathLibrary.MakeRotator` 0.0 0.0 _returnvalue_yaw)))
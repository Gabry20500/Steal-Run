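; Player character Blueprint that adds a slide and a hold-to-extend jump.
; Holding C sets IsSliding and runs a timeline that animates capsule half-height, reversing on release.
; Jump drives curve-scaled upward impulses through a timeline timed by JumpTime, stopped on release.
; Tick doubles gravity while descending and sets InJump, which blocks new jumps only during descent.
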(event `Key|C`
  (params (Key :type "Key Structure"))
  (:`Pressed`
    (set `self.IsSliding` true)
    (bind (_direction _setcapsuleheight) (`Timeline|SetCapsuleHeight` :!via `PlayFromStart` :!label _label)
      (:`Update`
        (`|ExecutionSequence`
          (:`then_0`
            (`CapsuleComponent.SetCapsuleHalfHeight` (`self.CapsuleComponent`) _setcapsuleheight true))))))
  (:`Released`
    (set `self.IsSliding` false)
    (goto _label :!via `Reverse`)))

(event `InputAction|Jump`
  (params (Key :type "Key Structure"))
  (:`Pressed`
    (if (not (`self.InJump`))
      (`TimelineComponent.SetPlayRate` (`self.JumpTimeline`) (/ 1.0 (`self.JumpTime`)))
      (bind (_direction _jumptrack) (`Timeline|JumpTimeline` :!via `PlayFromStart` :!label _label_2)
        (:`Update`
          (`CharacterMovementComponent.AddImpulse` (`self.CharacterMovement`) (`KismetMathLibrary.MakeVector` 0.0 0.0 (* _jumptrack (`self.JumpForce`))) false)))))
  (:`Released`
    (goto _label_2 :!via `Stop`)))

(event `self.ReceiveTick`
  (params (DeltaSeconds :type "Float (single-precision)"))
  (bind _charactermovement (`self.CharacterMovement`))
  (bind _charactermovement_2 (`self.CharacterMovement`))
  (bind (_velocity_x _velocity_y _velocity_z) (`KismetMathLibrary.BreakVector` (`MovementComponent.Velocity` _charactermovement_2)))
  (if (and (`NavMovementComponent.IsFalling` _charactermovement_2) (< _velocity_z 0.0))
    (set `self.InJump` true)
    (set `CharacterMovementComponent.GravityScale` 2.0 _charactermovement)
    (else
      (set `self.InJump` false)
      (set `CharacterMovementComponent.GravityScale` 1.0 _charactermovement))))

(fn `UserConstructionScript`)
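; Security camera enemy that sweeps up and down and alerts every enemy when it sees the player.
; Two timelines alternately lerp the actor's pitch between two angles, pausing briefly at each end.
; Pawn sensing sets the hasSeenPlayer blackboard key on all BP_BaseEnemy AI controllers through ChangeChaseValue.
; A delayed RemoveTarget event clears that key a few seconds later, and seeing a non-player pawn clears it immediately.
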(event `self.ReceiveBeginPlay`
  ;[1 1 1] Camera movement
  (`self.CameraMovement`))

(event `CameraMovement`
  (bind (_returnvalue_roll _returnvalue_pitch _returnvalue_yaw) (`KismetMathLibrary.BreakRotator` (`self.K2_GetActorRotation`)))
  (bind (_returnvalue_roll_2 _returnvalue_pitch_2 _returnvalue_yaw_2) (`KismetMathLibrary.BreakRotator` (`self.K2_GetActorRotation`)))
  ;[1 1 1] Camera movement
  (bind (_direction _0_1) (`Timeline|Camera movement` :!label _label)
    (:`Update`
      (`self.K2_SetActorRotation` (`KismetMathLibrary.MakeRotator` _returnvalue_roll_2 (`KismetMathLibrary.Lerp` _returnvalue_pitch_2 -50.0 _0_1) _returnvalue_yaw_2)))
    (:`Finished`
      (set `self.positiveRotation?` false)
      (`KismetSystemLibrary.Delay` 1.0)
      (bind (_direction_2 _0_1_2) (`Timeline|Timeline` :!via `PlayFromStart`)
        (:`Update`
          (`self.K2_SetActorRotation` (`KismetMathLibrary.MakeRotator` _returnvalue_roll (`KismetMathLibrary.Lerp` _returnvalue_pitch -70.0 _0_1_2) _returnvalue_yaw)))
        (:`Finished`
          (set `self.positiveRotation?` true)
          (`KismetSystemLibrary.Delay` 1.0)
          (goto _label :!via `PlayFromStart`))))))

(event `Remove target`
  ;[1 1 1] ChasePlayer
  (if (== (`self.PlayerReference`) (`self.As BP Player Character`))
    (`KismetSystemLibrary.Delay` 3.0)
    (`self.ChangeChaseValue` false)))

(event `self.PawnSensing.OnSeePawn`
  (params (Pawn :type "Pawn Object Reference"))
  ;[1 1 1] ChasePlayer
  (bind _asbp_player_character (cast `/Game/Player/BP_PlayerCharacter` Pawn)
    (:`then`
      (set `self.PlayerReference` _asbp_player_character)
      (set `self.As BP Player Character` _asbp_player_character)
      (`self.ChangeChaseValue` true)
      (`self.Remove target`))
    (:`CastFailed`
      (set `self.As BP Player Character` _asbp_player_character)
      (`self.ChangeChaseValue` false))))

(fn `ChangeChaseValue`
  (params (`ChasePlayer?` :type Boolean))
  (bind _outactors (`GameplayStatics.GetAllActorsOfClass` "/Game/Enemies/BaseAnemy/BP_BaseEnemy.BP_BaseEnemy_C"))
  (bind _output_get (set `self.AllEnemies` _outactors))
  (for _array_element _output_get
    (`BlackboardComponent.SetValueAsBool` (`AIBlueprintHelperLibrary.GetBlackboard` (`AIBlueprintHelperLibrary.GetAIController` _array_element)) "hasSeenPlayer" `ChasePlayer?`)))

(fn `UserConstructionScript`)
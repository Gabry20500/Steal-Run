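; Paper2D player character with crouch, variable-height jump and wall jump.
; Crouch drives capsule half-height through a timeline, while holding jump applies timeline-shaped upward force until release or timeline end.
; Each tick switches gravity between rising and falling unless on a wall, and traces along the flipbook's forward vector while airborne.
; A wall hit damps velocity toward zero and turns jump into a launch along the actor's right vector plus upward.
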(event `InputAction|Crunch`
  (params (Key :type "Key Structure"))
  (:`Pressed`
    (set `self.IsCrunched` true)
    (bind (_direction _setcapsuleheight) (`Timeline|SetCapsuleHeight` :!via `PlayFromStart` :!label _label)
      (:`Update`
        (`|ExecutionSequence`
          (:`then_0`
            (`CapsuleComponent.SetCapsuleHalfHeight` (`self.CapsuleComponent`) _setcapsuleheight true))))))
  (:`Released`
    (set `self.IsCrunched` false)
    (goto _label :!via `Reverse`)))

(event `InputAction|Jump`
  (params (Key :type "Key Structure"))
  (:`Pressed`
    (if (`self.WallJump?`)
      (`self.LaunchCharacter` (+ (* (`self.GetActorRightVector`) (`self.WallJumpForce`)) (0.0 0.0 1000.0)) true true)
      (elif (not (`NavMovementComponent.IsFalling` (`self.CharacterMovement`)))
        (`TimelineComponent.SetPlayRate` (`self.JumpTimeline`) (/ 1.0 (`self.JumpTime`)))
        (bind (_direction _jumptrack) (`Timeline|JumpTimeline` :!via `PlayFromStart` :!label _label_2)
          (:`Update`
            (`CharacterMovementComponent.AddForce` (`self.CharacterMovement`) (`KismetMathLibrary.MakeVector` 0.0 0.0 (* _jumptrack (`self.JumpForce`)))))))))
  (:`Released`
    (goto _label_2 :!via `Stop`)))

(event `self.ReceiveTick`
  (params (DeltaSeconds :type "Float (single-precision)"))
  (bind _paperflipbook (`self.PaperFlipbook`))
  (bind _charactermovement (`self.CharacterMovement`))
  (bind _returnvalue (`SceneComponent.K2_GetComponentLocation` _paperflipbook))
  (`self.SetGravityScale`)
  (if (`NavMovementComponent.IsFalling` (`self.CharacterMovement`))
    (bind (_outhit _returnvalue_2) (`KismetSystemLibrary.LineTraceSingle` _returnvalue (+ _returnvalue (* (`SceneComponent.GetForwardVector` _paperflipbook) (`self.WallCeckDistance`))) "TraceTypeQuery3"))
    (if _returnvalue_2
      (set `self.WallJump?` true)
      (set `MovementComponent.Velocity` (`KismetMathLibrary.VInterpTo_Constant` (`MovementComponent.Velocity` _charactermovement) (0.0 0.0 0.0) (`GameplayStatics.GetWorldDeltaSeconds`) 800.0) _charactermovement)
      (else
        (set `self.WallJump?` false :!label _label_3)))
    (else
      (goto _label_3))))

(fn `SetGravityScale`
  (bind _charactermovement (`self.CharacterMovement`))
  (bind (_velocity_x _velocity_y _velocity_z) (`KismetMathLibrary.BreakVector` (`MovementComponent.Velocity` (`self.CharacterMovement`))))
  (if (`self.WallJump?`)
    _
    (elif (and (`NavMovementComponent.IsFalling` (`self.CharacterMovement`)) (< _velocity_z 0.0))
      (set `CharacterMovementComponent.GravityScale` (`self.GravityScaleFall`) _charactermovement)
      (else
        (set `CharacterMovementComponent.GravityScale` (`self.GravityScaleJump`) _charactermovement)))))

(fn `UserConstructionScript`)
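; Side-scrolling follow camera that tracks the default pawn in Y and Z at a fixed world X set by XOffset.
; BeginPlay finds the pawn, positions and aims the camera once, then becomes the player's view target.
; Each Tick, dead-zone functions move the camera only when the pawn leaves the margin.
; A non-zero FixedZValue locks height; otherwise the downward Z check uses YDeadZone rather than ZDeadZone.
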(event `self.ReceiveBeginPlay`
  ;[1 1 1] Get Player Reference and set camera position
  (bind _returnvalue (`GameplayStatics.GetActorOfClass` (`GameModeBase.DefaultPawnClass` (`GameplayStatics.GetGameMode`))))
  (bind _output_get (set `self.ActorToFollow` _returnvalue))
  (bind (_returnvalue_x _returnvalue_y _returnvalue_z) (`KismetMathLibrary.BreakVector` (`self.K2_GetActorLocation` _output_get)))
  (bind _output_get_2 (set `self.CameraY` _returnvalue_y))
  (if (!= (`self.FixedZValue`) 0.0)
    (set `self.CameraZ` (`self.FixedZValue`))
    (else
      (bind _output_get_3 (set `self.CameraZ` (+ _returnvalue_z (`self.ZDeadZone`))))))
  (`self.K2_SetActorLocation` (`KismetMathLibrary.MakeVector` (`self.XOffset`) _output_get_2 _output_get_3))
  (`self.K2_SetActorRotation` (`KismetMathLibrary.FindLookAtRotation` (`self.K2_GetActorLocation`) (`self.K2_GetActorLocation` (`self.ActorToFollow`))))
  (`PlayerController.SetViewTargetWithBlend` (`GameplayStatics.GetPlayerController` 0) self 0.0 "VTBlend_Linear" 0.0 false))

(event `self.ReceiveTick`
  (params (DeltaSeconds :type "Float (single-precision)"))
  (bind _newy (`self.GetNewYValue`))
  (set `self.CameraY` _newy)
  (bind _new_z (`self.GetNewZValue`))
  (set `self.CameraZ` _new_z)
  (`self.K2_SetActorLocation` (`KismetMathLibrary.MakeVector` (`self.XOffset`) (`self.CameraY`) (`self.CameraZ`))))

(fn `GetNewYValue`
  (returns (NewY :type "Float (double-precision)"))
  (bind (_returnvalue_x _returnvalue_y) (`KismetMathLibrary.BreakVector` (`self.K2_GetActorLocation`)))
  (bind (_returnvalue_x_2 _returnvalue_y_2) (`KismetMathLibrary.BreakVector` (`self.K2_GetActorLocation`)))
  (bind (_returnvalue_x_3 _returnvalue_y_3) (`KismetMathLibrary.BreakVector` (`self.K2_GetActorLocation` (`self.ActorToFollow`))))
  (bind (_returnvalue_x_4 _returnvalue_y_4) (`KismetMathLibrary.BreakVector` (`self.K2_GetActorLocation` (`self.ActorToFollow`))))
  (bind _returnvalue (- _returnvalue_y_4 (`self.YDeadZone`)))
  (bind _returnvalue_2 (+ _returnvalue_y_3 (`self.YDeadZone`)))
  (if (> _returnvalue _returnvalue_y_2)
    (return _returnvalue)
    (elif (< _returnvalue_2 _returnvalue_y)
      (return _returnvalue_2)
      (else
        (return (`self.CameraY`))))))

(fn `GetNewZValue`
  (returns (`New Z` :type "Float (double-precision)"))
  (bind (_returnvalue_x _returnvalue_y _returnvalue_z) (`KismetMathLibrary.BreakVector` (`self.K2_GetActorLocation`)))
  (bind (_returnvalue_x_2 _returnvalue_y_2 _returnvalue_z_2) (`KismetMathLibrary.BreakVector` (`self.K2_GetActorLocation`)))
  (bind (_returnvalue_x_3 _returnvalue_y_3 _returnvalue_z_3) (`KismetMathLibrary.BreakVector` (`self.K2_GetActorLocation` (`self.ActorToFollow`))))
  (bind (_returnvalue_x_4 _returnvalue_y_4 _returnvalue_z_4) (`KismetMathLibrary.BreakVector` (`self.K2_GetActorLocation` (`self.ActorToFollow`))))
  (bind _returnvalue (- _returnvalue_z_4 (`self.ZDeadZone`)))
  (bind _returnvalue_2 (+ _returnvalue_z_3 (`self.YDeadZone`)))
  (if (!= (`self.FixedZValue`) 0.0)
    (return (`self.FixedZValue`))
    (elif (> _returnvalue _returnvalue_z_2)
      (return _returnvalue)
      (elif (< _returnvalue_2 _returnvalue_z)
        (return _returnvalue_2)
        (else
          (return (`self.CameraZ`)))))))

(fn `UserConstructionScript`)
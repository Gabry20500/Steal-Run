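; BP_BaseEnemy is an enemy Blueprint that flags player sightings for its AI.
; PawnSensing stores a seen BP_PlayerCharacter, sets the blackboard key hasSeenPlayer to true and calls RemoveTarget.
; RemoveTarget compares the two stored player references, then clears the key after a fixed Delay, which repeat sightings do not restart.
; Seeing any other pawn clears the key immediately.
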(event `Remove target`
  (if (== (`self.PlayerReference`) (`self.As BP Player Character`))
    (`KismetSystemLibrary.Delay` 3.0)
    (`BlackboardComponent.SetValueAsBool` (`AIBlueprintHelperLibrary.GetBlackboard` (`AIBlueprintHelperLibrary.GetAIController` self)) "hasSeenPlayer" false)))

(event `self.PawnSensing.OnSeePawn`
  (params (Pawn :type "Pawn Object Reference"))
  (bind _asbp_player_character (cast `/Game/Scripts/Player/BP_PlayerCharacter` Pawn)
    (:`then`
      (set `self.PlayerReference` _asbp_player_character)
      (set `self.As BP Player Character` _asbp_player_character)
      (`BlackboardComponent.SetValueAsBool` (`AIBlueprintHelperLibrary.GetBlackboard` (`AIBlueprintHelperLibrary.GetAIController` self)) "hasSeenPlayer" true)
      (`self.Remove target`))
    (:`CastFailed`
      (set `self.As BP Player Character` null)
      (`BlackboardComponent.SetValueAsBool` (`AIBlueprintHelperLibrary.GetBlackboard` (`AIBlueprintHelperLibrary.GetAIController` self)) "hasSeenPlayer" false))))

(fn `UserConstructionScript`)
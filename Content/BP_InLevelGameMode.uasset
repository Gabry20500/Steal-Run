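; In-level game mode that runs a two-phase objective round, handling the player HUD, timer display and win/lose outcomes.
; Tick watches the primary-object flag and fires the second phase once, adding a run widget; its music and enemy hooks are unfinished.
; Losing shows a paused game-over screen, or teleports the player if the object is held and time remains.
; Resetting the first phase clears the flag and enemy targets, then opens the win level.
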(event `self.ReceiveTick`
  (params (DeltaSeconds :type "Float (single-precision)"))
  (bind _returnvalue (`self.GetPrimaryObjectObtained`))
  (if _returnvalue
    (`/Engine/EditorBlueprintResources/StandardMacros.DoOnce` false
      (:`Completed`
        (`self.SetSecondPhase` (`KismetMathLibrary.Conv_BoolToDouble` _returnvalue))))))

(fn `ActivateUI`
  (bind _returnvalue (`|CreateWidget` "/Game/BluePrints/Player/UI/WB_UIPlayer.WB_UIPlayer_C"))
  (`UserWidget.AddToViewport` _returnvalue 0)
  (set `self.UIRef` _returnvalue))

(fn `ChangeUI`
  (params (NewWidjet :type "UserWidget Class Reference") (`Show Mouse Cursor` :type Boolean) (bPaused :type Boolean))
  (`WidgetLayoutLibrary.RemoveAllWidgets`)
  (bind _returnvalue (`|CreateWidget` NewWidjet))
  (`UserWidget.AddToViewport` _returnvalue 0)
  (set `PlayerController.bShowMouseCursor` `Show Mouse Cursor` (`GameplayStatics.GetPlayerController` 0))
  (`GameplayStatics.SetGamePaused` bPaused))

(fn `LoseScreen`
  (params (`Timer ended` :type Boolean))
  (if (`self.GetPrimaryObjectObtained`)
    (if `Timer ended`
      (`self.ChangeUI` "/Game/BluePrints/MenuScript/BPW_GameOverScreen.BPW_GameOverScreen_C" true true)
      (else
        (`self.K2_SetActorLocation` (`GameplayStatics.GetPlayerCharacter` 0) (1115.0 17625.0 145.0) false false)))
    (else
      (`self.ChangeUI` "/Game/BluePrints/MenuScript/BPW_GameOverScreen.BPW_GameOverScreen_C" true true))))

(fn `ResetFirstPahse`
  (`/Engine/EditorBlueprintResources/StandardMacros.DoOnce` false
    (:`Completed`
      (`|ExecutionSequence`
        (:`then_0`
          (`self.SetPrimaryObjectObtained` false))
        (:`then_1`
          (bind _outactors (`GameplayStatics.GetAllActorsOfClass` "/Game/BluePrints/Enemies/BaseAnemy/BP_BaseEnemy.BP_BaseEnemy_C"))
          (for _array_element _outactors
            (`/Game/BluePrints/Enemies/BaseAnemy/BP_BaseEnemy.Remove target` _array_element)))
        (:`then_2`
          (`self.WinScreen`))))))

(fn `SetSecondPhase`
  (params (Value :type "Float (double-precision)"))
  (bind _returnvalue (`|CreateWidget` "/Game/BluePrints/Player/UI/WB_Run.WB_Run_C"))
  (`UserWidget.AddToViewport` _returnvalue 0)
  (bind _outactors (`GameplayStatics.GetAllActorsWithTag` "MusicAudio"))
  (for _array_element _outactors
    (bind _asfmodambient_sound (cast `FMODAmbientSound` _array_element))))

(fn `SetTimerValue`
  (params (Minutes :type Integer) (Seconds :type Integer) (MilliSeconds :type Integer))
  (bind _uiref (`self.UIRef`))
  (set `/Game/BluePrints/Player/UI/WB_UIPlayer.Minutes` Minutes _uiref)
  (set `/Game/BluePrints/Player/UI/WB_UIPlayer.Seconds` Seconds _uiref)
  (set `/Game/BluePrints/Player/UI/WB_UIPlayer.MilliSeconds` MilliSeconds _uiref))

(fn `UserConstructionScript`)

(fn `WinScreen`
  (`GameplayStatics.OpenLevel` "EndLevelWin"))
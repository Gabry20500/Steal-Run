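; MusicAudio is an actor that drives adaptive in-level music through an FMOD audio component.
; Every Tick it casts to the player character and sets the "Objects" parameter from its collectable counter.
; It then checks the in-level game mode and sets "Collected" while the primary object is obtained, never resetting it here.
; ChangeVolume forwards a given value to the "Volume" parameter.
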(event `self.ReceiveTick`
  (params (DeltaSeconds :type "Float (single-precision)"))
  (bind _asbp_player_zdcharacter (cast `/Game/BluePrints/Player/BP_PlayerZDCharacter` (`GameplayStatics.GetPlayerPawn` 0)))
  (`FMODAudioComponent.SetParameter` (`self.FMODAudio`) "Objects" (`KismetMathLibrary.Conv_IntToDouble` (`PlayerZDCharacter.CollectableCounter` _asbp_player_zdcharacter)))
  (bind _asbp_in_level_game_mode (cast `/Game/BP_InLevelGameMode` (`GameplayStatics.GetGameMode`)))
  (bind _returnvalue (`InLevelGameMode.GetPrimaryObjectObtained` _asbp_in_level_game_mode))
  (if _returnvalue
    (`FMODAudioComponent.SetParameter` (`self.FMODAudio`) "Collected" (`KismetMathLibrary.Conv_BoolToDouble` _returnvalue))))

(fn `ChangeVolume`
  (params (Value :type "Float (single-precision)"))
  (`FMODAudioComponent.SetParameter` (`self.FMODAudio`) "Volume" Value))

(fn `UserConstructionScript`)
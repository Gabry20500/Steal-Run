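; BP_InterDoor1 is an interactable door actor that registers itself with the player character when approached.
; Entering its Box trigger caches the BP_PlayerZDCharacter, sets the door as that player's interactable object, flags interaction and reveals a Widget component.
; Leaving the box clears the flag and hides the widget, but does not reset the player's interactable reference.
; The door contains no opening logic of its own.
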(event `self.Box.OnComponentBeginOverlap`
  (params (OverlappedComponent :type "PrimitiveComponent Object Reference") (OtherActor :type "Actor Object Reference") (OtherComp :type "PrimitiveComponent Object Reference") (OtherBodyIndex :type Integer) (bFromSweep :type Boolean) (SweepResult :type "HitResult Structure (by ref)"))
  (bind _asbp_player_zdcharacter (cast `/Game/BluePrints/Player/BP_PlayerZDCharacter` OtherActor))
  (bind _output_get (set `self.PlayerRef` _asbp_player_zdcharacter))
  (`PlayerZDCharacter.SetInteractableObject` _output_get self)
  (`PlayerZDCharacter.SetbIsInteracting` _output_get true)
  (`SceneComponent.SetHiddenInGame` (`self.Widget`) false false))

(event `self.Box.OnComponentEndOverlap`
  (params (OverlappedComponent :type "PrimitiveComponent Object Reference") (OtherActor :type "Actor Object Reference") (OtherComp :type "PrimitiveComponent Object Reference") (OtherBodyIndex :type Integer))
  (cast `/Game/BluePrints/Player/BP_PlayerZDCharacter` OtherActor)
  (`PlayerZDCharacter.SetbIsInteracting` (`self.PlayerRef`) false)
  (`SceneComponent.SetHiddenInGame` (`self.Widget`) true false))

(fn `UserConstructionScript`)
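; BP_LaserTrap is a single-use trap actor that temporarily takes away the player's control when triggered.
; A Box overlap waits briefly, casts to BP_PlayerZDCharacter, then disables that character's input.
; The TrapDuration timeline serves as a timer, with its play rate scaled by the inverse of TrapDurationTime.
; When the timeline finishes, input is restored and the trap destroys itself.
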(event `self.Box.OnComponentBeginOverlap`
  (params (OverlappedComponent :type "PrimitiveComponent Object Reference") (OtherActor :type "Actor Object Reference") (OtherComp :type "PrimitiveComponent Object Reference") (OtherBodyIndex :type Integer) (bFromSweep :type Boolean) (SweepResult :type "HitResult Structure (by ref)"))
  (bind _returnvalue (`GameplayStatics.GetPlayerController` 0))
  (`KismetSystemLibrary.Delay` 0.2)
  (bind _asbp_player_zdcharacter (cast `/Game/BluePrints/Player/BP_PlayerZDCharacter` OtherActor))
  (`self.DisableInput` _asbp_player_zdcharacter _returnvalue)
  (`TimelineComponent.SetPlayRate` (`self.TrapDuration`) (/ 1.0 (`self.TrapDurationTime`)))
  (`Timeline|TrapDuration` :!via `PlayFromStart`
    (:`Finished`
      (`self.EnableInput` _asbp_player_zdcharacter _returnvalue)
      (`self.K2_DestroyActor`))))

(fn `UserConstructionScript`)
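; Base enemy pawn that detects the player by sight or sound and triggers the game mode's lose screen when its capsule touches them.
; Pawn sensing and a hearing overlap that matches "SoundBox"-tagged components set the blackboard's hasSeenPlayer flag.
; A three-second delay then clears that flag and inStartPos, which is set true on BeginPlay as the start location is saved.
; GetAllTimePlayerPos also sets hasSeenPlayer, without the timeout, and prints a call counter.
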(event `Remove target`
  (`KismetSystemLibrary.Delay` 3.0)
  (`BlackboardComponent.SetValueAsBool` (`self.BlackBoardComponent`) "hasSeenPlayer" false)
  (`BlackboardComponent.SetValueAsBool` (`self.BlackBoardComponent`) "inStartPos" false))

(event `self.PawnSensing.OnSeePawn`
  (params (Pawn :type "Pawn Object Reference"))
  (`BlackboardComponent.SetValueAsBool` (`self.BlackBoardComponent`) "hasSeenPlayer" true)
  (`self.Remove target`))

(event `GetAllTimePlayerPos`
  (bind _result (`/Engine/EditorBlueprintResources/StandardMacros.IncrementInt` (`self.C`))
    (:`  `
      (bind _output_get (set `self.C` _result))
      (`KismetSystemLibrary.PrintString` (`KismetStringLibrary.Conv_IntToString` _output_get))
      (`BlackboardComponent.SetValueAsBool` (`self.BlackBoardComponent`) "hasSeenPlayer" true))))

(event `self.CapsuleComponent.OnComponentBeginOverlap`
  (params (OverlappedComponent :type "PrimitiveComponent Object Reference") (OtherActor :type "Actor Object Reference") (OtherComp :type "PrimitiveComponent Object Reference") (OtherBodyIndex :type Integer) (bFromSweep :type Boolean) (SweepResult :type "HitResult Structure (by ref)"))
  (cast `/Game/BluePrints/Player/BP_PlayerZDCharacter` OtherActor)
  (bind _asbp_in_level_game_mode (cast `/Game/BP_InLevelGameMode` (`GameplayStatics.GetGameMode`)))
  (`/Game/BP_InLevelGameMode.LoseScreen` _asbp_in_level_game_mode false))

(event `self.ReceiveBeginPlay`
  (set `self.StartPos` (`self.K2_GetActorLocation`))
  (bind _output_get (set `self.BlackBoardComponent` (`AIBlueprintHelperLibrary.GetBlackboard` (`AIBlueprintHelperLibrary.GetAIController` self))))
  (`BlackboardComponent.SetValueAsBool` _output_get "inStartPos" true))

(event `self.EnemyEaring.OnComponentBeginOverlap`
  (params (OverlappedComponent :type "PrimitiveComponent Object Reference") (OtherActor :type "Actor Object Reference") (OtherComp :type "PrimitiveComponent Object Reference") (OtherBodyIndex :type Integer) (bFromSweep :type Boolean) (SweepResult :type "HitResult Structure (by ref)"))
  (cast `/Game/BluePrints/Player/BP_PlayerZDCharacter` OtherActor)
  (for _array_element (`ActorComponent.ComponentTags` OtherComp)
    (if (== _array_element "SoundBox")
      (`self.ChasePlayer` true))))

(fn `ChasePlayer`
  (params (BoolValue :type Boolean))
  (`BlackboardComponent.SetValueAsBool` (`AIBlueprintHelperLibrary.GetBlackboard` null) "hasSeenPlayer" BoolValue)
  (`KismetSystemLibrary.PrintString` "GetPosition")
  (`self.Remove target`))

(fn `UserConstructionScript`)
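; BP_Button is a menu button that keeps its visual style in sync with mouse hover and keyboard focus.
; Start sets a looping timer that polls CheckFocus instead of binding hover or focus events.
; CheckFocus gives a hovered button keyboard focus and the mouse style, so mouse and keyboard share one selection.
; Otherwise it applies the selected or unselected key style based on keyboard focus.
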(fn `CheckFocus`
  (if (`self.IsHovered`)
    (`self.SetKeyboardFocus`)
    (`self.SetStyle` (`self.MouseStyle`))
    (else
      (`self.SetStyle` (select `bool` (`self.HasKeyboardFocus`) :`false` (`self.KeyNotSelected`) :`true` (`self.KeySelected`))))))

(fn `Start`
  (`KismetSystemLibrary.K2_SetTimer` null "CheckFocus" 0.1 true))
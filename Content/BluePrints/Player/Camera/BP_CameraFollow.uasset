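; BP_CameraFollow is a side-on camera actor that becomes the view target and follows the player along Y and Z.
; Each Tick applies dead zones, optional fixed axis values and an optional minimum Y.
; An active camera trigger, passed via SetNewOffsets, pauses following while a duration-scaled timeline lerps to new offsets.
; The timeline reverses when the player isn't facing right, and on finish commits the new or old settings by direction.
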(event `self.ReceiveBeginPlay`
  ;[1 1 1] Get Player Reference and set camera position
  (bind _returnvalue (`GameplayStatics.GetActorOfClass` (`GameModeBase.DefaultPawnClass` (`GameplayStatics.GetGameMode`))))
  (bind _output_get (set `self.ActorToFollow` _returnvalue))
  (bind (_returnvalue_x _returnvalue_y _returnvalue_z) (`KismetMathLibrary.BreakVector` (`self.K2_GetActorLocation` _output_get)))
  (bind _output_get_2 (set `self.CameraY` _returnvalue_y))
  (if (!= (`self.FixedZValue`) 0.0)
    (set `self.CameraZ` (`self.FixedZValue`))
    (else
      (bind _output_get_3 (set `self.CameraZ` (+ _returnvalue_z (`self.ZDeadZone`) (`self.ZOffset`))))))
  (`self.K2_SetActorLocation` (`KismetMathLibrary.MakeVector` (`self.XOffset`) _output_get_2 _output_get_3))
  (set `self.MinCamY` (`self.CameraY`))
  (`self.K2_SetActorRotation` (`KismetMathLibrary.FindLookAtRotation` (`self.K2_GetActorLocation`) (`self.K2_GetActorLocation` (`self.ActorToFollow`))))
  (`PlayerController.SetViewTargetWithBlend` (`GameplayStatics.GetPlayerController` 0) self 0.0 "VTBlend_Linear" 0.0 false))

(event `self.ReceiveTick`
  (params (DeltaSeconds :type "Float (single-precision)"))
  ;[1 1 1] Camera position control for trigger
  (if (!= (`self.Reference CT`) null)
    (if (`CamTrigger.IsInTrigger` (`self.Reference CT`))
      (if (not (`self.Lerping`))
        (`/Engine/EditorBlueprintResources/StandardMacros.DoOnce` false :!label _label
          (:`Completed`
            (`self.PlayTimeline`))))
      (else
        (if (not (`self.Lerping`)) :!label _label_2
          (bind _newy (`self.GetNewYValue`))
          (set `self.CameraY` _newy)
          (bind _new_z (`self.GetNewZValue`))
          (set `self.CameraZ` _new_z)
          (`self.K2_SetActorLocation` (`KismetMathLibrary.MakeVector` (`self.XOffset`) (`self.CameraY`) (`self.CameraZ`))))))
    (else
      (goto _label_2))))

(event `ResetDoOnce`
  ;[1 1 1] Camera position control for trigger
  (goto _label :!via `Reset`))

(event `PlayTimeline`
  (bind _reference_ct (`self.Reference CT`))
  (bind (_oldstartpos_x _oldstartpos_y _oldstartpos_z) (`KismetMathLibrary.BreakVector` (`CamTrigger.OldStartPos` _reference_ct)))
  ;[1 1 1] Camera Lerp
  (set `self.StartLoc` (`CamTrigger.OldStartPos` (`self.Reference CT`)))
  (`TimelineComponent.SetPlayRate` (`self.LerpTimeline`) (/ 1.0 (`CamTrigger.LerpDuration` (`self.Reference CT`))))
  (bind _asbp_player_zdcharacter (cast `/Game/BluePrints/Player/BP_PlayerZDCharacter` (`self.ActorToFollow`)))
  (if (`|EnumEquality` (`PlayerZDCharacter.PlayerDirection` _asbp_player_zdcharacter) "Right")
    (bind (_direction _timeline) (`Timeline|LerpTimeline` :!via `PlayFromStart` :!label _label_3)
      (:`Update`
        (bind (_lerpedx _lerpedy _lerpedz _ydz _zdz) (`self.Set New Camera Pos` _timeline)))
      (:`Finished`
        (set `self.Lerping` false)
        (set `CamTrigger.IsInTrigger` false (`self.Reference CT`))
        (`self.ResetDoOnce`)
        (bind _asbp_player_zdcharacter_2 (cast `/Game/BluePrints/Player/BP_PlayerZDCharacter` (`self.ActorToFollow`)))
        (if (`|EnumEquality` (`PlayerZDCharacter.PlayerDirection` _asbp_player_zdcharacter_2) "Right")
          (set `self.XOffset` _lerpedx)
          (bind _output_get (set `self.CameraY` _lerpedy))
          (bind _output_get_2 (set `self.CameraZ` _lerpedz))
          (set `self.YDeadZone` _ydz)
          (set `self.ZDeadZone` _zdz)
          (set `self.FixedZValue` _output_get_2)
          (set `self.FixedYValue` _output_get)
          (else
            (set `self.XOffset` _oldstartpos_x)
            (set `self.CameraY` _oldstartpos_y)
            (set `self.CameraZ` _oldstartpos_z)
            (set `self.YDeadZone` (`CamTrigger.OldYDeadZone` _reference_ct))
            (set `self.ZDeadZone` (`CamTrigger.OldZDeadZone` _reference_ct))
            (set `self.FixedZValue` (`CamTrigger.OldFixedZ` _reference_ct))
            (set `self.FixedYValue` (`CamTrigger.OldFixedY` _reference_ct))))))
    (else
      (goto _label_3 :!via `ReverseFromEnd`))))

(fn `GetNewYValue`
  (returns (NewY :type "Float (double-precision)"))
  (bind (_returnvalue_x _returnvalue_y) (`KismetMathLibrary.BreakVector` (`self.K2_GetActorLocation`)))
  (bind (_returnvalue_x_2 _returnvalue_y_2) (`KismetMathLibrary.BreakVector` (`self.K2_GetActorLocation`)))
  (bind (_returnvalue_x_3 _returnvalue_y_3) (`KismetMathLibrary.BreakVector` (`self.K2_GetActorLocation` (`self.ActorToFollow`))))
  (bind (_returnvalue_x_4 _returnvalue_y_4) (`KismetMathLibrary.BreakVector` (`self.K2_GetActorLocation` (`self.ActorToFollow`))))
  (bind (_returnvalue_x_5 _returnvalue_y_5) (`KismetMathLibrary.BreakVector` (`self.K2_GetActorLocation` (`self.ActorToFollow`))))
  (bind _returnvalue (- _returnvalue_y_4 (`self.YDeadZone`)))
  (bind _returnvalue_2 (+ _returnvalue_y_3 (`self.YDeadZone`)))
  (if (`self.LockMinCameraY`)
    (if (<= _returnvalue_y_5 (`self.MinCamY`))
      (return (+ (`self.MinCamY`) (`self.YDeadZone`)))
      (else
        _)))
  (if (!= 0.0 (`self.FixedYValue`))
    (return (`self.FixedYValue`))
    (elif (> _returnvalue _returnvalue_y_2)
      (return _returnvalue)
      (elif (< _returnvalue_2 _returnvalue_y)
        (return _returnvalue_2)
        (else
          (return (`self.CameraY`)))))))

(fn `GetNewZValue`
  (returns (`New Z` :type "Float (double-precision)"))
  (bind (_returnvalue_x _returnvalue_y _returnvalue_z) (`KismetMathLibrary.BreakVector` (`self.K2_GetActorLocation`)))
  (bind (_returnvalue_x_2 _returnvalue_y_2 _returnvalue_z_2) (`KismetMathLibrary.BreakVector` (`self.K2_GetActorLocation`)))
  (bind (_returnvalue_x_3 _returnvalue_y_3 _returnvalue_z_3) (`KismetMathLibrary.BreakVector` (`self.K2_GetActorLocation` (`self.ActorToFollow`))))
  (bind (_returnvalue_x_4 _returnvalue_y_4 _returnvalue_z_4) (`KismetMathLibrary.BreakVector` (`self.K2_GetActorLocation` (`self.ActorToFollow`))))
  (bind _returnvalue (- _returnvalue_z_4 (`self.ZDeadZone`)))
  (bind _returnvalue_2 (+ _returnvalue_z_3 (`self.YDeadZone`)))
  (if (!= (`self.FixedZValue`) 0.0)
    (return (`self.FixedZValue`))
    (elif (> _returnvalue _returnvalue_z_2)
      (return _returnvalue)
      (elif (< _returnvalue_2 _returnvalue_z)
        (return _returnvalue_2)
        (else
          (return (`self.CameraZ`)))))))

(fn `Set New Camera Pos`
  (params (Alpha :type "Float (double-precision)"))
  (returns (LerpedX :type "Float (double-precision)") (LerpedY :type "Float (double-precision)") (LerpedZ :type "Float (double-precision)") (YDz :type "Float (double-precision)") (ZDz :type "Float (double-precision)"))
  (locals (LerpedZOff :type "Float (double-precision)" :default 0.0) (`Lerped XOff` :type "Float (double-precision)" :default 0.0) (LerpedYOff :type "Float (double-precision)"))
  (bind (_startloc_x _startloc_y _startloc_z) (`KismetMathLibrary.BreakVector` (`self.StartLoc`)))
  (bind (_startloc_x_2 _startloc_y_2) (`KismetMathLibrary.BreakVector` (`self.StartLoc`)))
  (bind _startloc_x_3 (`KismetMathLibrary.BreakVector` (`self.StartLoc`)))
  (set `self.Lerping` true)
  (`|ExecutionSequence`
    (:`then_0`
      (set `local.Lerped XOff` (`KismetMathLibrary.Lerp` _startloc_x_3 (`self.New XOffset`) (`local.Alpha`)))
      (set `local.LerpedZOff` (`KismetMathLibrary.Lerp` _startloc_z (`self.New ZOffset`) (`local.Alpha`)))
      (set `local.LerpedYOff` (`KismetMathLibrary.Lerp` _startloc_y_2 (`self.New YOffset`) (`local.Alpha`)))
      (`self.K2_SetActorLocation` (`KismetMathLibrary.MakeVector` (`local.Lerped XOff`) (`local.LerpedYOff`) (`local.LerpedZOff`)))
      (return (`local.Lerped XOff`) (`local.LerpedYOff`) (`local.LerpedZOff`) (`self.New YDeadZone`) (`self.New ZDeadZone`)))))

(fn `SetNewOffsets`
  (params (NewXOffset :type "Float (double-precision)") (NewYOffset :type "Float (double-precision)") (NewZOffset :type "Float (double-precision)") (NewYDeadZone :type "Float (double-precision)") (NewZDeadZone :type "Float (double-precision)") (ReferenceCT :type "CamTrigger Object Reference"))
  (set `self.New XOffset` NewXOffset)
  (set `self.New YOffset` NewYOffset)
  (set `self.New ZOffset` NewZOffset)
  (set `self.New YDeadZone` NewYDeadZone)
  (set `self.New ZDeadZone` NewZDeadZone)
  (set `self.Reference CT` ReferenceCT))

(fn `UserConstructionScript`)
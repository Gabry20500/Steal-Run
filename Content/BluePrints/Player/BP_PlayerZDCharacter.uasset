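; PaperZD player character Blueprint handling jump, wall jump, crouch toggle and climb animation, and setting Hologram on its ability manager child actor at start.
; Jumping applies timeline-driven force until released, while gravity scale switches between jump and fall values.
; While airborne, a forward trace each tick detects walls, damps velocity and enables a launch-based wall jump.
; Mantle overlap triggers the climb animation, and animation states change through PaperZD node jumps.
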(event `InputAction|Jump`
  (params (Key :type "Key Structure"))
  (:`Pressed`
    (if (`self.WallJump?`)
      (`PaperZDAnimInstance.JumpToNode` (`PaperZDAnimationComponent.AnimInstance` (`self.AnimationComponent`)) "AirBorne" "None")
      (`self.LaunchCharacter` (+ (* (`self.GetActorRightVector`) (`self.WallJumpForce`)) (0.0 0.0 1000.0)) true true)
      (elif (not (`NavMovementComponent.IsFalling` (`self.CharacterMovement`)))
        (`TimelineComponent.SetPlayRate` (`self.JumpTimeline`) (/ 1.0 (`self.JumpTime`)))
        (`PaperZDAnimInstance.JumpToNode` (`PaperZDAnimationComponent.AnimInstance` (`self.AnimationComponent`)) "AirBorne" "None")
        (bind (_direction _jumptrack) (`Timeline|JumpTimeline` :!via `PlayFromStart` :!label _label)
          (:`Update`
            (`CharacterMovementComponent.AddForce` (`self.CharacterMovement`) (`KismetMathLibrary.MakeVector` 0.0 0.0 (* _jumptrack (`self.JumpForce`)))))))))
  (:`Released`
    (goto _label :!via `Stop`)))

(event `InputAction|Crunch`
  (params (Key :type "Key Structure"))
  (:`Pressed`
    (`/Engine/EditorBlueprintResources/StandardMacros.FlipFlop`
      (:`A`
        (set `self.IsInCrunch` true)
        (`self.Crouch`)
        (`PaperZDAnimInstance.JumpToNode` (`PaperZDAnimationComponent.AnimInstance` (`self.AnimationComponent`)) "Crouch" "None"))
      (:`B`
        (set `self.IsInCrunch` false)
        (`self.UnCrouch`)
        (`PaperZDAnimInstance.JumpToNode` (`PaperZDAnimationComponent.AnimInstance` (`self.AnimationComponent`)) "RunAnim" "None")))))

(event `self.ReceiveTick`
  (params (DeltaSeconds :type "Float (single-precision)"))
  (bind _charactermovement (`self.CharacterMovement`))
  (bind _returnvalue (`SceneComponent.K2_GetComponentLocation` (`self.CapsuleComponent`)))
  (`|ExecutionSequence`
    (:`then_0`
      (`self.SetGravityScale`))
    (:`then_1`
      (if (`NavMovementComponent.IsFalling` (`self.CharacterMovement`))
        (bind (_outhit _returnvalue_2) (`KismetSystemLibrary.LineTraceSingle` _returnvalue (+ _returnvalue (* (`SceneComponent.GetForwardVector` (`self.Sprite`)) (`self.WallCeckDistance`))) "TraceTypeQuery3"))
        (if _returnvalue_2
          (set `self.WallJump?` true)
          (set `MovementComponent.Velocity` (`KismetMathLibrary.VInterpTo_Constant` (`MovementComponent.Velocity` _charactermovement) (0.0 0.0 0.0) (`GameplayStatics.GetWorldDeltaSeconds`) 800.0) _charactermovement)
          (`PaperZDAnimInstance.JumpToNode` (`PaperZDAnimationComponent.AnimInstance` (`self.AnimationComponent`)) "WallAction" "None")
          (else
            (set `self.WallJump?` false :!label _label_2)))
        (else
          (goto _label_2))))
    (:`then_2`
      (if (`self.bIsOverlappingWithMantle`)
        (set `self.CanMantle` true)
        (`/Engine/EditorBlueprintResources/StandardMacros.DoOnce` false :!label _label_3
          (:`Completed`
            (`PaperZDAnimInstance.JumpToNode` (`PaperZDAnimationComponent.AnimInstance` (`self.AnimationComponent`)) "Climb" "None")
            (set `self.bIsOverlappingWithMantle` false)
            (goto _label_3 :!via `Reset`)))))))

(event `self.OnWalkingOffLedge`
  (params (PreviousFloorImpactNormal :type "Vector Structure (by ref)") (PreviousFloorContactNormal :type "Vector Structure (by ref)") (PreviousLocation :type "Vector Structure (by ref)") (TimeDelta :type "Float (single-precision)"))
  (`PaperZDAnimInstance.JumpToNode` (`PaperZDAnimationComponent.AnimInstance` (`self.AnimationComponent`)) "AirBorne" "None"))

(event `self.ReceiveBeginPlay`
  (bind _asbpa_ability_manager (cast `/Game/BluePrints/Player/BPA_AbilityManager` (`ChildActorComponent.ChildActor` (`self.BPA_AbilityManager`))))
  (`AbilitiesManager.SetAbility` _asbpa_ability_manager "Hologram"))

(fn `SetGravityScale`
  (bind _charactermovement (`self.CharacterMovement`))
  (bind (_velocity_x _velocity_y _velocity_z) (`KismetMathLibrary.BreakVector` (`MovementComponent.Velocity` (`self.CharacterMovement`))))
  (if (`self.WallJump?`)
    _
    (elif (and (`NavMovementComponent.IsFalling` (`self.CharacterMovement`)) (< _velocity_z 0.0))
      (set `CharacterMovementComponent.GravityScale` (`self.GravityScaleFall`) _charactermovement)
      (else
        (set `CharacterMovementComponent.GravityScale` (`self.GravityScaleJump`) _charactermovement)))))

(fn `UserConstructionScript`)